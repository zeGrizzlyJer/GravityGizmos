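; Activatable door for the physics game that slides between a closed and an open position.
; Activate plays the SwitchActivate timeline, whose alpha drives UpdatePosition to lerp the Collider between the StartPos and OpenPos world locations without sweeping.
; Deactivate reverses the timeline to close the door, but only when CanDeactivate is set.
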(event EventActivate
  (bind _lerpalpha (Timeline|SwitchActivate Play)
    (:Update
      (Utilities|UpdatePosition _lerpalpha))))

(event EventDeactivate
  (if (Variables|Default|GetCanDeactivate)
    (bind _lerpalpha (Timeline|SwitchActivate Reverse)
      (:Update
        (Utilities|UpdatePosition _lerpalpha)))))

(fn ConstructionScript)
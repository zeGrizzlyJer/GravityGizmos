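; Actor component that highlights its owning actor by toggling Render Custom Depth on the owner's static mesh component, which it caches on BeginPlay.
; Highlight turns the effect on, unless RequiresVision is set and InView is false, in which case it turns it off.
; LightsOut clears the highlight unconditionally.
; InView is only read here, not computed.
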(event EventBeginPlay
  (Variables|Default|SetStaticMesh (Actor|GetComponentbyClass (Components|GetOwner) "/Script/Engine.StaticMeshComponent")))

(fn Highlight
  (if (Variables|Default|GetRequiresVision)
    (if (Variables|Default|GetInView)
      (Variables|Default|SetIsHighlighted true :!label _label)
      (else
        (bind _output_get (Variables|Default|SetIsHighlighted false))))
    (else
      (goto _label)))
  (Rendering|SetRenderCustomDepth (Variables|Default|GetStaticMesh) _output_get))

(fn LightsOut
  (bind _output_get (Variables|Default|SetIsHighlighted false))
  (Rendering|SetRenderCustomDepth (Variables|Default|GetStaticMesh) _output_get))
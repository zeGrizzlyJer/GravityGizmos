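; BP_Pickup is a physics pickup actor that the third-person player character can detect when nearby.
; On BeginPlay it initializes its ACPickupable component with itself and its static mesh.
; A Box trigger adds or removes the actor from BP_ThirdPersonCharacter's pickup list on overlap begin and end, printing debug text each time.
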(event OnComponentBeginOverlap(Box)
  (params (OverlappedComponent :type Primitive%20Component%20Object%20Reference) (OtherActor :type Actor%20Object%20Reference) (OtherComp :type Primitive%20Component%20Object%20Reference) (OtherBodyIndex :type Integer) (bFromSweep :type Boolean) (SweepResult :type Hit%20Result%20Structure%20%28by%20ref%29))
  (bind _asbp_third_person_character (Utilities|Casting|CastToBP_ThirdPersonCharacter OtherActor))
  (Default|AddPickuptoList _asbp_third_person_character self)
  (Development|PrintText "Object Near Player"))

(event OnComponentEndOverlap(Box)
  (params (OverlappedComponent :type Primitive%20Component%20Object%20Reference) (OtherActor :type Actor%20Object%20Reference) (OtherComp :type Primitive%20Component%20Object%20Reference) (OtherBodyIndex :type Integer))
  (bind _asbp_third_person_character (Utilities|Casting|CastToBP_ThirdPersonCharacter OtherActor))
  (Default|RemovePickupfromList _asbp_third_person_character self)
  (Development|PrintText "Object Leaving Player"))

(event EventBeginPlay
  (Default|Initialize (Variables|Default|GetAC_Pickupable) self (Variables|Default|GetStaticMesh)))

(fn ConstructionScript)
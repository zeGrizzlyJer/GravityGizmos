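; Actor component that returns its owning actor to a saved respawn point in the physics game.
; SetRespawnTransform stores a transform in the BP_GameInstance Respawns map, keyed by the owner, and prints a debug message.
; Respawn teleports the owner to that location and rotation, then, if the root is a primitive component, zeroes its physics velocities and drops it through any AC_Grabbable component.
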(event EventBeginPlay)

(event EventTick
  (params (DeltaSeconds :type Float%20%28single-precision%29)))

(fn Respawn
  (bind _self self)
  (bind _self_2 self)
  (bind _returnvalue (Components|GetOwner _self_2))
  (bind _returnvalue_2 (Components|GetOwner _self))
  (bind _returnvalue_3 (Actor|GetComponentbyClass _returnvalue "/Game/_PhysicsGameContent/Blueprints/AC_Grabbable.AC_Grabbable_C"))
  (bind _asbp_game_instance (Utilities|Casting|CastToBP_GameInstance (Game|GetGameInstance)))
  (Transformation|SetActorLocationAndRotation _returnvalue_2 (.location (.Value (Utilities|Map|Find (Variables|/Game/_PhysicsGameContent/Blueprints/Modes/BP_GameInstance.BP_GameInstance_C|GetRespawns _asbp_game_instance) _returnvalue_2))) (.rotation (.Value (Utilities|Map|Find (Variables|/Game/_PhysicsGameContent/Blueprints/Modes/BP_GameInstance.BP_GameInstance_C|GetRespawns _asbp_game_instance) _returnvalue_2))) false true)
  (bind _asprimitive_component (Utilities|Casting|CastToPrimitiveComponent (Variables|/Script/Engine.Actor|GetRootComponent _returnvalue_2)))
  (Physics|SetPhysicsLinearVelocity _asprimitive_component "0, 0, 0" false "None")
  (Class|PrimitiveComponent|SetPhysicsAngularVelocityinDegrees _asprimitive_component "0, 0, 0" false "None")
  (Utilities|IsValid _returnvalue_3
    (:Is%20Valid
      (Default|Drop _returnvalue_3))))

(fn SetRespawnTransform
  (params (Respawn :type Transform))
  (bind _asbp_game_instance (Utilities|Casting|CastToBP_GameInstance (Game|GetGameInstance)))
  (Utilities|Map|Add (Variables|/Game/_PhysicsGameContent/Blueprints/Modes/BP_GameInstance.BP_GameInstance_C|GetRespawns _asbp_game_instance) (Components|GetOwner self) Respawn)
  (Development|PrintString (Utilities|String|Append "Respawn set on: " (Utilities|GetObjectName (Components|GetOwner self))) true true "(R=1.000000,G=0.000000,B=0.885502,A=1.000000)"))
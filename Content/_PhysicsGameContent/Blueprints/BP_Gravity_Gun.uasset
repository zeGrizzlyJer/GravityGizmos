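; Gravity gun that lets the player grab, drop and rotate physics objects.
; Left input line-traces forward from an offset along the aim and calls Grab on a hit physics-simulating object's AC_Grabbable, if nothing is held.
; Right input calls Drop on the third-person character's GrabbedItem, while holding Reload sets that character's IsRotating flag.
; A CheckIfHasGrabbable macro gates grab and drop on the character's IsGrabbing state.
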(event EventBeginPlay
  (|CallParentFunction) ; This node is disabled and will not be called.\nDrag off pins to build functionality.
)

(event EventLeftStart
  (params (Location :type Vector :default "0, 0, 0") (Rotation :type Rotator :default "0, 0, 0"))
  (bind _returnvalue (Math|Vector|GetForwardVector Rotation))
  ;[0.1954 1 0.2807] Grab Item
  (Development|PrintText "Attempt Left Start")
  (Utilities|CheckifHasGrabbable
    (:DoesNot
      (bind (_outhit _returnvalue_2) (Collision|LineTraceByChannel (+ Location (* _returnvalue 4e+02)) (+ Location (* _returnvalue 1e+03)) "TraceTypeQuery1" false (Utilities|Array|MakeArray (Game|Player|GetPlayerPawn 0)) "ForDuration"))
      (if _returnvalue_2
        (if (Physics|IsSimulatingPhysics (.HitComponent (Collision|BreakHitResult _outhit)) "None")
          (Utilities|IsValid (Actor|GetComponentbyClass (.HitActor (Collision|BreakHitResult _outhit)) "/Game/_PhysicsGameContent/Blueprints/AC_Grabbable.AC_Grabbable_C")
            (:Is%20Valid
              (Default|Grab (Actor|GetComponentbyClass (.HitActor (Collision|BreakHitResult _outhit)) "/Game/_PhysicsGameContent/Blueprints/AC_Grabbable.AC_Grabbable_C")))
            (:Is%20Not%20Valid
              (Development|PrintString "Not a valid grabbable object"))))))))

(event EventRightStart
  ;[1 0.1403 0.214] Drop Item
  (Development|PrintText "Attempt Right Start")
  (Utilities|CheckifHasGrabbable
    (:HasPickup
      (bind _asbp_third_person_character (Utilities|Casting|CastToBP_ThirdPersonCharacter (Game|Player|GetPlayerPawn 0)))
      (Default|Drop (Actor|GetComponentbyClass (Variables|/Game/ThirdPerson/Blueprints/BP_ThirdPersonCharacter.BP_ThirdPersonCharacter_C|GetGrabbedItem _asbp_third_person_character) "/Game/_PhysicsGameContent/Blueprints/AC_Grabbable.AC_Grabbable_C")))))

(event EventReloadStart
  ;[0.2143 0.1162 0.6677] Rotate Item
  (Development|PrintText "Attempt Reload Start")
  (bind _asbp_third_person_character (Utilities|Casting|CastToBP_ThirdPersonCharacter (Game|Player|GetPlayerPawn 0)))
  (Variables|/Game/ThirdPerson/Blueprints/BP_ThirdPersonCharacter.BP_ThirdPersonCharacter_C|SetIsRotating _asbp_third_person_character true))

(event EventRightEnd
  (Development|PrintText "Attempt Right End"))

(event EventLeftEnd
  (Development|PrintText "Attempt Left End"))

(event EventReloadEnd
  ;[0.2143 0.1162 0.6677] Rotate Item
  (Development|PrintText "Attempt Reload End")
  (bind _asbp_third_person_character (Utilities|Casting|CastToBP_ThirdPersonCharacter (Game|Player|GetPlayerPawn 0)))
  (Variables|/Game/ThirdPerson/Blueprints/BP_ThirdPersonCharacter.BP_ThirdPersonCharacter_C|SetIsRotating _asbp_third_person_character false))

(fn ConstructionScript
  (|CallParentFunction))
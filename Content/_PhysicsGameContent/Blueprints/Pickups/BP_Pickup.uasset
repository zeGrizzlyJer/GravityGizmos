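; BP_Pickup is a physics-game pickup actor that the third-person character can detect, with pickup, respawn and highlight behavior split into components.
; BeginPlay initializes the pickupable component with the static mesh and stores the starting transform in the respawn component.
; Box overlaps add or remove it from the character's pickup list, highlighting it only when first in that list.
; Pickup clears the highlight, drop and reload-end events are empty, and GetMass exposes the mesh's mass.
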(event OnComponentBeginOverlap(Box)
  (params (OverlappedComponent :type Primitive%20Component%20Object%20Reference) (OtherActor :type Actor%20Object%20Reference) (OtherComp :type Primitive%20Component%20Object%20Reference) (OtherBodyIndex :type Integer) (bFromSweep :type Boolean) (SweepResult :type Hit%20Result%20Structure%20%28by%20ref%29))
  (bind _asbp_third_person_character (Utilities|Casting|CastToBP_ThirdPersonCharacter OtherActor))
  (Default|AddPickuptoList _asbp_third_person_character self)
  (if (== (Utilities|Array|Get(acopy) (Variables|/Game/ThirdPerson/Blueprints/BP_ThirdPersonCharacter.BP_ThirdPersonCharacter_C|GetPickups _asbp_third_person_character)) (Variables|Default|GetAC_Pickupable))
    (Default|Highlight (Variables|Default|GetAC_Highlight))
    (else
      (Development|PrintText "Object Near Player"))))

(event OnComponentEndOverlap(Box)
  (params (OverlappedComponent :type Primitive%20Component%20Object%20Reference) (OtherActor :type Actor%20Object%20Reference) (OtherComp :type Primitive%20Component%20Object%20Reference) (OtherBodyIndex :type Integer))
  (bind _asbp_third_person_character (Utilities|Casting|CastToBP_ThirdPersonCharacter OtherActor))
  (Default|RemovePickupfromList _asbp_third_person_character self)
  (Default|LightsOut (Variables|Default|GetAC_Highlight)))

(event EventOnPickup
  (Default|LightsOut (Variables|Default|GetAC_Highlight)))

(event EventOnDrop)

(event EventReloadEnd)

(event EventBeginPlay
  (bind _self self)
  (Default|Initialize (Variables|Default|GetAC_Pickupable) _self (Variables|Default|GetStaticMesh))
  (Default|SetRespawnTransform (Variables|Default|GetAC_Respawn) (Transformation|GetActorTransform _self)))

(fn ConstructionScript)

(fn GetMass
  (return (Physics|GetMass (Variables|Default|GetStaticMesh))))
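; BP_Jetpack is a pickup that gives the player pawn left and right thrusters while carried.
; On pickup it sends thruster locations and force to the pawn through BPI_Jetpack and shows its UI; dropping zeroes the force and hides it.
; Left and right input events forward thrust on/off to the pawn and toggle Niagara effects.
; A middle effect plays only while both thrusters are active.
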(event EventBeginPlay
  ;[0.1302 0.1302 0.1302] Initialize UI
  (|CallParentFunction)
  (bind _returnvalue (UserInterface|CreateWidget "/Game/_PhysicsGameContent/Blueprints/UI/BP_JetpackUI.BP_JetpackUI_C"))
  (Variables|Default|SetJetpackUI _returnvalue))

(event EventLeftThruston
  ;[0.1284 1 0.1274] Trigger Jetpack Interactions
  (Utilities|ActivateLeftThrust)
  (bind _asbpi_jetpack (Utilities|Casting|CastToBPI_Jetpack (Game|Player|GetPlayerPawn 0)))
  (Default|LeftThruston _asbpi_jetpack))

(event EventOnDrop
  ;[0 1 0.7305] On Pickup & Drop
  (bind _asbpi_jetpack (Utilities|Casting|CastToBPI_Jetpack (Game|Player|GetPlayerPawn 0)))
  (Default|UpdateThrustForce _asbpi_jetpack "0, 0, 0")
  (Utilities|DeactivateThrusters)
  (Widget|RemovefromParent (Variables|Default|GetJetpackUI)))

(event EventDeactivateThrust
  ;[0.1284 1 0.1274] Trigger Jetpack Interactions
  (Utilities|DeactivateThrusters))

(event EventLeftThrustOff
  ;[0.1284 1 0.1274] Trigger Jetpack Interactions
  (Utilities|DeactivateLeftThrust)
  (bind _asbpi_jetpack (Utilities|Casting|CastToBPI_Jetpack (Game|Player|GetPlayerPawn 0)))
  (Default|LeftThrustOff _asbpi_jetpack))

(event EventLeftStart
  (params (Location :type Vector :default "0, 0, 0") (Rotation :type Rotator :default "0, 0, 0"))
  ;[1 0.1933 0.2192] Pickupable -> Jetpack Interaction Conversion
  (Development|PrintText "Attempt Left Burner")
  (CallFunction|LeftThruston))

(event EventLeftEnd
  ;[1 0.1933 0.2192] Pickupable -> Jetpack Interaction Conversion
  (Development|PrintText "Deactivate Left Burner")
  (CallFunction|LeftThrustOff))

(event EventRightStart
  ;[1 0.1933 0.2192] Pickupable -> Jetpack Interaction Conversion
  (Development|PrintText "Attempt Right Burner")
  (CallFunction|RightThruston))

(event EventRightEnd
  ;[1 0.1933 0.2192] Pickupable -> Jetpack Interaction Conversion
  (Development|PrintText "Deactivate Right Burner")
  (CallFunction|RightThrustOff))

(event EventRightThruston
  ;[0.1284 1 0.1274] Trigger Jetpack Interactions
  (Utilities|ActivateRightThrust)
  (bind _asbpi_jetpack (Utilities|Casting|CastToBPI_Jetpack (Game|Player|GetPlayerPawn 0)))
  (Default|RightThruston _asbpi_jetpack))

(event EventRightThrustOff
  ;[0.1284 1 0.1274] Trigger Jetpack Interactions
  (Utilities|DeactivateRightThrust)
  (bind _asbpi_jetpack (Utilities|Casting|CastToBPI_Jetpack (Game|Player|GetPlayerPawn 0)))
  (Default|RightThrustOff _asbpi_jetpack))

(event EventOnPickup
  ;[0 1 0.7305] On Pickup & Drop
  (bind _asbpi_jetpack (Utilities|Casting|CastToBPI_Jetpack (Game|Player|GetPlayerPawn 0)))
  (Default|UpdateThrusterLocation _asbpi_jetpack (Variables|Default|GetLeftThrustLocation) (Variables|Default|GetRightThrustLocation))
  (Default|UpdateThrustForce _asbpi_jetpack (Variables|Default|GetThrustForce))
  (UserInterface|Viewport|AddtoViewport (Variables|Default|GetJetpackUI) 0))

(fn ConstructionScript
  (|CallParentFunction))

(fn GetMass
  (return (Variables|Default|GetTriggerMass)))
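; An actor component that lets a physics-simulated object be picked up, carried and dropped.
; Initialize stores the owning object and its static mesh, and an IsCarried flag guards against repeated pickups or drops.
; Pickup disables physics and collision, then snaps the object to a socket on the host.
; Drop detaches it, moves it to the given socket's location and rotation, then restores collision and physics.
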(fn Pickup
  (params (HostObject :type Scene%20Component%20Object%20Reference) (SocketName :type Name))
  (bind _staticmesh (Variables|Components|GetStaticMesh))
  (if (not (Variables|Components|GetIsCarried))
    (Physics|SetSimulatePhysics _staticmesh false)
    (Collision|SetCollisionEnabled _staticmesh "NoCollision")
    (Transformation|AttachComponentToComponent (Variables|Components|GetAttachedObject) HostObject SocketName "SnapToTarget" "SnapToTarget" "SnapToTarget" true)
    (Variables|Components|SetIsCarried true)))

(fn Drop
  (params (HostMesh :type Scene%20Component%20Object%20Reference) (SocketName :type Name))
  (bind _attachedobject (Variables|Components|GetAttachedObject))
  (bind _staticmesh (Variables|Components|GetStaticMesh))
  (if (Variables|Components|GetIsCarried)
    (Transformation|DetachFromActor _attachedobject "KeepRelative" "KeepRelative" "KeepRelative")
    (Transformation|SetActorLocationAndRotation _attachedobject (Transformation|GetSocketLocation HostMesh SocketName) (Transformation|GetSocketRotation HostMesh SocketName))
    (Variables|Components|SetIsCarried false)
    (Collision|SetCollisionEnabled _staticmesh "QueryAndPhysics")
    (Physics|SetSimulatePhysics _staticmesh true)))

(fn Initialize
  (params (ParentObject :type Actor%20Object%20Reference) (ParentMesh :type Static%20Mesh%20Component%20Object%20Reference))
  (Variables|Components|SetAttachedObject ParentObject)
  (Variables|Components|SetStaticMesh ParentMesh))
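; Actor component that makes its owner a physics object the player character can grab, drop or blast.
; Grab disables mesh physics and attaches the owner to the character's GravityArm, updating its grab state.
; Drop and Blast restore physics, clear that state and call DetachFromActor on the character; Blast also resets velocities and applies an impulse.
; OnGrab and OnDrop events forward to the owner through BPI_Grabbable.
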(event EventBeginPlay
  (bind _self self)
  (bind _returnvalue (Components|GetOwner _self))
  (CallFunction|Initialize _self _returnvalue (Actor|GetComponentbyClass _returnvalue "/Script/Engine.StaticMeshComponent")))

(event EventOnDrop
  (bind _asbpi_grabbable (Utilities|Casting|CastToBPI_Grabbable (Variables|Components|GetAttachedObject)))
  (Default|OnDrop _asbpi_grabbable))

(event EventOnGrab
  (bind _asbpi_grabbable (Utilities|Casting|CastToBPI_Grabbable (Variables|Components|GetAttachedObject)))
  (Default|OnGrab _asbpi_grabbable))

(fn Initialize
  (params (Actor :type Actor%20Object%20Reference) (StaticMesh :type Static%20Mesh%20Component%20Object%20Reference))
  (Variables|Components|SetAttachedObject Actor)
  (Variables|Components|SetStaticMesh StaticMesh))

(fn Grab
  (bind _self self)
  (bind _returnvalue (Components|GetOwner _self))
  (Development|PrintString "GRAB" true true "(R=0.000000,G=1.000000,B=0.364652,A=1.000000)")
  (bind _asbp_third_person_character (Utilities|Casting|CastToBP_ThirdPersonCharacter (Game|Player|GetPlayerPawn 0)))
  (Variables|/Game/ThirdPerson/Blueprints/BP_ThirdPersonCharacter.BP_ThirdPersonCharacter_C|SetGrabbedItem _asbp_third_person_character _returnvalue)
  (Variables|/Game/ThirdPerson/Blueprints/BP_ThirdPersonCharacter.BP_ThirdPersonCharacter_C|SetIsGrabbing _asbp_third_person_character true)
  (Physics|SetSimulatePhysics (Variables|Components|GetStaticMesh) false)
  (Transformation|AttachComponentToComponent _returnvalue (Variables|/Game/ThirdPerson/Blueprints/BP_ThirdPersonCharacter.BP_ThirdPersonCharacter_C|GetGravityArm _asbp_third_person_character) "None" "SnapToTarget" "KeepWorld" "KeepWorld" true)
  (Class|BPIGrabbable|OnGrab(Message) self))

(fn Drop
  (Development|PrintString "DROP" true true "(R=1.000000,G=0.000000,B=0.139113,A=1.000000)")
  (bind _asbp_third_person_character (Utilities|Casting|CastToBP_ThirdPersonCharacter (Pawn|GetControlledPawn (Game|GetPlayerController 0))))
  (Variables|/Game/ThirdPerson/Blueprints/BP_ThirdPersonCharacter.BP_ThirdPersonCharacter_C|SetGrabbedItem _asbp_third_person_character 0)
  (Variables|/Game/ThirdPerson/Blueprints/BP_ThirdPersonCharacter.BP_ThirdPersonCharacter_C|SetIsGrabbing _asbp_third_person_character false)
  (Physics|SetSimulatePhysics (Variables|Components|GetStaticMesh) true)
  (Transformation|DetachFromActor _asbp_third_person_character "KeepRelative" "KeepRelative" "KeepRelative")
  (Class|BPIGrabbable|OnDrop(Message) self))

(fn Blast
  (params (BlastForce :type Vector))
  (Development|PrintString "BLAST" true true "(R=0.179259,G=0.087880,B=1.000000,A=1.000000)")
  (bind _asbp_third_person_character (Utilities|Casting|CastToBP_ThirdPersonCharacter (Pawn|GetControlledPawn (Game|GetPlayerController 0))))
  (Variables|/Game/ThirdPerson/Blueprints/BP_ThirdPersonCharacter.BP_ThirdPersonCharacter_C|SetGrabbedItem _asbp_third_person_character 0)
  (Variables|/Game/ThirdPerson/Blueprints/BP_ThirdPersonCharacter.BP_ThirdPersonCharacter_C|SetIsGrabbing _asbp_third_person_character false)
  (Physics|SetSimulatePhysics (Variables|Components|GetStaticMesh) true)
  (Transformation|DetachFromActor _asbp_third_person_character "KeepRelative" "KeepRelative" "KeepRelative")
  (Class|PrimitiveComponent|SetAllPhysicsLinearVelocity (Variables|Components|GetStaticMesh) (Math|Vector|MakeVector 0.0 0.0 0.0) false)
  (Class|PrimitiveComponent|SetAllPhysicsAngularVelocityinDegrees (Variables|Components|GetStaticMesh) (Math|Vector|MakeVector 0.0 0.0 0.0) false)
  (Physics|AddImpulse (Variables|Components|GetStaticMesh) BlastForce "None" false)
  (Class|BPIGrabbable|OnDrop(Message) self))
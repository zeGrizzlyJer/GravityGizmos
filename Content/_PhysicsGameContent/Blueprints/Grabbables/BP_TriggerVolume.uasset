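; BP_TriggerVolume is a grabbable physics object that highlights when the third-person character enters its trigger sphere.
; Without a vision requirement it highlights on overlap through ACHighlight, and lights go out on exit.
; With one, a 0.2-second delay loop line-traces the mesh along the follow camera's forward vector to set InView, checking player distance.
; GetMass exposes the mesh's mass, and an unfinished timer approach sits unused.
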(event OnComponentBeginOverlap(TriggerVolume)
  (params (OverlappedComponent :type Primitive%20Component%20Object%20Reference) (OtherActor :type Actor%20Object%20Reference) (OtherComp :type Primitive%20Component%20Object%20Reference) (OtherBodyIndex :type Integer) (bFromSweep :type Boolean) (SweepResult :type Hit%20Result%20Structure%20%28by%20ref%29))
  (bind _asbp_third_person_character (Utilities|Casting|CastToBP_ThirdPersonCharacter OtherActor))
  (bind _output_get (Variables|Default|SetPlayerRef _asbp_third_person_character))
  (if (Variables|/Game/_PhysicsGameContent/Blueprints/AC_Highlight.AC_Highlight_C|GetRequiresVision (Variables|Default|GetAC_Highlight))
    (Variables|Default|SetCheckingForVision true)
    (CallFunction|DetermineVision _output_get :!label _label)
    (if (Variables|Default|GetCanBeHighlighted)
      (Utilities|FlowControl|Delay 0.2)
      (goto _label)
      (else
        (Variables|Default|SetCheckingForVision false)
        (Default|LightsOut (Variables|Default|GetAC_Highlight))))
    (else
      (Default|Highlight (Variables|Default|GetAC_Highlight)))))

(event OnComponentEndOverlap(TriggerVolume)
  (params (OverlappedComponent :type Primitive%20Component%20Object%20Reference) (OtherActor :type Actor%20Object%20Reference) (OtherComp :type Primitive%20Component%20Object%20Reference) (OtherBodyIndex :type Integer))
  (Utilities|Casting|CastToBP_ThirdPersonCharacter OtherActor)
  (if (Variables|/Game/_PhysicsGameContent/Blueprints/AC_Highlight.AC_Highlight_C|GetRequiresVision (Variables|Default|GetAC_Highlight))
    (Variables|Default|SetCheckingForVision false))
  (Default|LightsOut (Variables|Default|GetAC_Highlight)))

(fn ConstructionScript)

(fn DetermineVision
  (params (Player :type BP%20Third%20Person%20Character%20Object%20Reference))
  (bind _triggervolume (Variables|Default|GetTriggerVolume))
  (bind _followcamera (Variables|/Game/ThirdPerson/Blueprints/BP_ThirdPersonCharacter.BP_ThirdPersonCharacter_C|GetFollowCamera Player))
  (bind _returnvalue (Transformation|GetWorldLocation _followcamera))
  (bind _sphereradius (Variables|/Script/Engine.SphereComponent|GetSphereRadius _triggervolume))
  (if (Variables|Default|GetCheckingForVision)
    (bind _returnvalue_2 (Collision|LineTraceComponent (Variables|Default|GetStaticMesh) _returnvalue (+ _returnvalue (* (Math|Vector|GetForwardVector _followcamera) (+ _sphereradius 4e+02))) true false false))
    (Variables|/Game/_PhysicsGameContent/Blueprints/AC_Highlight.AC_Highlight_C|SetInView (Variables|Default|GetAC_Highlight) _returnvalue_2)
    (Default|Highlight (Variables|Default|GetAC_Highlight))
    (Variables|Default|SetCheckingForVision (<= (Math|Float|Absolute(Float) (Math|Vector|Distance(Vector) (Transformation|GetActorLocation Player) (Transformation|GetActorLocation self))) (+ _sphereradius 5e+01))))
  (return))

(fn GetMass
  (return (Physics|GetMass (Variables|Default|GetStaticMesh))))
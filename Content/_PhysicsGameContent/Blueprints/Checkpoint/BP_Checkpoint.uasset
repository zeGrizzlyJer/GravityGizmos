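; BP_Checkpoint is a checkpoint pickup shown as a floppy disc mesh that spins continuously on Tick.
; When the third-person character overlaps its sphere, it plays a 2D sound and stores that character with the RespawnLocation transform in the game instance's Respawns map.
; It then sets the CheckpointOn flag and passes itself to the game instance's UpdateCheckpoint.
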(event OnComponentBeginOverlap(SphereCollision)
  (params (OverlappedComponent :type Primitive%20Component%20Object%20Reference) (OtherActor :type Actor%20Object%20Reference) (OtherComp :type Primitive%20Component%20Object%20Reference) (OtherBodyIndex :type Integer) (bFromSweep :type Boolean) (SweepResult :type Hit%20Result%20Structure%20%28by%20ref%29))
  (bind _asbp_third_person_character (Utilities|Casting|CastToBP_ThirdPersonCharacter OtherActor))
  (Audio|PlaySound2D "/Engine/EditorSounds/Notifications/CompileFailed.CompileFailed" 1.0 1.0 0.0 0 0)
  (bind _asbp_game_instance (Utilities|Casting|CastToBP_GameInstance (Game|GetGameInstance)))
  (Utilities|Map|Add (Variables|/Game/_PhysicsGameContent/Blueprints/Modes/BP_GameInstance.BP_GameInstance_C|GetRespawns _asbp_game_instance) _asbp_third_person_character (Transformation|GetWorldTransform (Variables|Default|GetRespawn%20Location)))
  (Variables|/Game/_PhysicsGameContent/Blueprints/Modes/BP_GameInstance.BP_GameInstance_C|SetCheckpointOn _asbp_game_instance true)
  (Default|UpdateCheckpoint _asbp_game_instance self))

(event EventTick
  (params (DeltaSeconds :type Float%20%28single-precision%29))
  (Transformation|AddLocalRotation (Variables|Default|GetfloppyDiscSM) (Math|Rotator|MakeRotator (* DeltaSeconds 5e+01) 0.0 0.0) false false))

(fn ConstructionScript)